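; BP_NPC is an AI-controlled character that shows its AI state on a floating icon and has a health component.
; On BeginPlay it caches the state widget from a child-actor icon and binds to its AIC_NPC controller's state updates, which play animations on that widget.
; Health change and depletion events only print debug messages.
; SetData applies the default patrol speed from its data to walk speed.
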(event OnHealthChanged(BP_HealthComponent)
  (params (NewHealth :type Float%20%28double-precision%29))
  (Development|PrintString (Utilities|String|Append "Health: " (Utilities|String|ToString(Float) NewHealth)) true true "(R=0.338521,G=1.000000,B=0.000000,A=1.000000)" 2.0 "Health"))

(event OnHealthDepleted(BP_HealthComponent)
  (Development|PrintString "Died" true true "(R=1.000000,G=0.144312,B=0.000000,A=1.000000)" 2.0 ""))

(event Custom|UpdatedState
  (params (State :type E_Awareness%20Enum :default "NewEnumerator0") (PlayAnimation :type Boolean) (Restore%20anim%20state :type Boolean))
  (Default|PlayStateAnimation (Variables|Default|GetFloating%20Icon%20Widget) State PlayAnimation Restore%20anim%20state))

(event EventBeginPlay
  (bind _asai_state_icon (Utilities|Casting|CastToAI_StateIcon (Variables|/Script/Engine.ChildActorComponent|GetChildActor (Variables|Default|GetAI_StateIcon))))
  (bind _output_get (Variables|Default|SetWBP%20Icon%20General _asai_state_icon))
  (bind _aswbp_enemy_state (Utilities|Casting|CastToWBP_EnemyState (UserInterface|GetUserWidgetObject (Variables|/Game/AI/AI_StateIcon.AI_StateIcon_C|GetWBP_State _output_get))))
  (Variables|Default|SetFloating%20Icon%20Widget _aswbp_enemy_state)
  (bind _asaic_npc (Utilities|Casting|CastToAIC_NPC (AI|GetAIController self)))
  (EventDispatchers|BindEventtoUpdatedState _asaic_npc (delegate Custom|UpdatedState)))

(event Collision|EventActorBeginOverlap
  (params (OtherActor :type Actor%20Object%20Reference)))

(event EventTick
  (params (DeltaSeconds :type Float%20%28single-precision%29)))

(fn ConstructionScript)

(fn SetData
  (Variables|/Script/Engine.CharacterMovementComponent|SetMaxWalkSpeed (Variables|Character|GetCharacterMovement) (Variables|/Game/AI/PDA_AI.PDA_AI_C|GetDefaultPatrolSpeed (Variables|Default|GetData))))