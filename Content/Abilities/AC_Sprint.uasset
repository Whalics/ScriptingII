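; Sprint ability component that switches the player's max walk speed between run and walk values from Data and toggles the sprint FOV.
; StartSprinting requires the player to be grounded and moving within a direction threshold, checked by dotting normalized velocity against actor forward.
; While sprinting, Tick stops it when that direction check fails on the ground, so sprint persists in the air.
; CanSprint still prints debug strings.
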(event EventBeginPlay
  (|CallParentFunction) ; This node is disabled and will not be called.\nDrag off pins to build functionality.
)

(event EventTick
  (params (DeltaSeconds :type Float%20%28single-precision%29))
  (if (Variables|Default|GetbIsSprinting)
    (CallFunction|UpdateSprint)))

(fn StartSprinting
  (bind _can_sprint_ (CallFunction|CanSprint?))
  (if _can_sprint_
    (Variables|/Script/Engine.CharacterMovementComponent|SetMaxWalkSpeed (Variables|/Script/Engine.Character|GetCharacterMovement (Variables|Default|GetPlayer)) (Variables|/Game/DataAssets/PDA_General.PDA_General_C|GetRun%20Speed (Variables|Default|GetData)))
    (Variables|Default|SetbIsSprinting true)
    (Default|SprintFOV (Variables|Default|GetPlayer))))

(fn StopSprinting
  (Variables|Default|SetbIsSprinting false)
  (Variables|/Script/Engine.CharacterMovementComponent|SetMaxWalkSpeed (Variables|/Script/Engine.Character|GetCharacterMovement (Variables|Default|GetPlayer)) (Variables|/Game/DataAssets/PDA_General.PDA_General_C|GetWalk%20Speed (Variables|Default|GetData)))
  (Default|UnSprintFOV (Variables|Default|GetPlayer)))

(fn CanSprint?
  (if (Utilities|IsFalling)
    (return false)
    (elif (Utilities|IsGrounded)
      (if (Utilities|GetMoveDir)
        (if (Utilities|IsMoving)
          (Development|PrintString "can sprint")
          (return true)
          (else
            (Development|PrintString "cant sprint")
            (return false)))
        (else
          (return false)))
      (else
        (return false)))))

(fn UpdateSprint
  (if (not (Utilities|GetMoveDir))
    (if (Utilities|IsGrounded)
      (CallFunction|StopSprinting))))