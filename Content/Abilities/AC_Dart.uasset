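; Dart ability component that readies a floating dart at the player's weapon spawn point and fires it as a projectile.
; Each tick the dart lerps toward that point and rotates toward a camera line trace hit, or the trace end.
; Holding past the data-defined zoom time sets Primed and zooms the camera.
; Firing replaces the dart with BP_DartProjectile, plays camera shake and ends the zoom if primed.
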(event EventTick
  (params (DeltaSeconds :type Float%20%28single-precision%29))
  (Utilities|IsValid (Variables|Default|GetDartInstance)
    (:Is%20Valid
      (CallFunction|SetDartTransform))))

(fn HoldZoom
  (params (Hold%20Time :type Float%20%28double-precision%29))
  (if (> Hold%20Time (Variables|/Game/DataAssets/PDA_Dart.PDA_Dart_C|GetZoomTime (Variables|Default|GetData)))
    (Variables|Default|SetbPrimed true)
    (Default|ZoomCamera (Variables|Default|GetPlayer))))

(fn Prime
  (bind _returnvalue (Game|SpawnActorfromClass (Variables|Default|GetDart) (Transformation|GetWorldTransform (Variables|/Game/FirstPerson/Blueprints/BP_FirstPersonCharacter.BP_FirstPersonCharacter_C|GetWeaponSpawnPoint (Variables|Default|GetPlayer))) "AlwaysSpawn" "MultiplyWithRoot" 0 0))
  (bind _output_get (Variables|Default|SetDartInstance _returnvalue))
  (return _output_get))

(fn FireProjectile
  (Development|PrintString "Fired")
  (Default|PlayCameraShake (Variables|Default|GetPlayer) "/Game/CameraShake/FireProjectile.FireProjectile_C")
  (Game|SpawnActorfromClass "/Game/Blueprints/BP_DartProjectile.BP_DartProjectile_C" (Transformation|GetActorTransform (Variables|Default|GetDartInstance)) "Undefined" "MultiplyWithRoot" 0 0)
  (Actor|DestroyActor (Variables|Default|GetDartInstance))
  (Variables|Default|SetDartInstance 0)
  (Utilities|Primed?
    (:true
      (Default|EndZoomCamera (Variables|Default|GetPlayer)))))

(fn LerptoPosition
  (return (Math|Vector|Lerp(Vector) (Transformation|GetActorLocation (Variables|Default|GetDartInstance)) (Transformation|GetWorldLocation (Variables|/Game/FirstPerson/Blueprints/BP_FirstPersonCharacter.BP_FirstPersonCharacter_C|GetWeaponSpawnPoint (Variables|Default|GetPlayer))) (Variables|/Game/DataAssets/PDA_Dart.PDA_Dart_C|GetFollowLerpAlpha (Variables|Default|GetData)))))

(fn SetProjectileRotation
  (bind _dartinstance (Variables|Default|GetDartInstance))
  (bind (_out _bhit) (Default|GetLineTracefromCamera (Variables|Default|GetPlayer) 5e+03 "TraceTypeQuery1"))
  (return (Math|Rotator|Lerp(Rotator) (Transformation|GetWorldRotation (Variables|/Game/Blueprints/BP_Dart.BP_Dart_C|GetShard _dartinstance)) (Math|Rotator|MakeRotator (.roll (Math|Rotator|FindLookatRotation (Transformation|GetActorLocation _dartinstance) (Math|Vector|SelectVector (.ImpactPoint (Collision|BreakHitResult _out)) (.TraceEnd (Collision|BreakHitResult _out)) _bhit))) (+ (.pitch (Math|Rotator|FindLookatRotation (Transformation|GetActorLocation _dartinstance) (Math|Vector|SelectVector (.ImpactPoint (Collision|BreakHitResult _out)) (.TraceEnd (Collision|BreakHitResult _out)) _bhit))) 0.0) (.yaw (Math|Rotator|FindLookatRotation (Transformation|GetActorLocation _dartinstance) (Math|Vector|SelectVector (.ImpactPoint (Collision|BreakHitResult _out)) (.TraceEnd (Collision|BreakHitResult _out)) _bhit)))) (Variables|/Game/DataAssets/PDA_Dart.PDA_Dart_C|GetRotateLerpAlpha (Variables|Default|GetData)) true)))

(fn SetDartTransform
  (Utilities|IsValid (Variables|Default|GetDartInstance)
    (:Is%20Valid
      (bind _returnvalue (CallFunction|SetProjectileRotation))
      (bind _returnvalue_2 (CallFunction|LerptoPosition))
      (Transformation|SetActorLocationAndRotation (Variables|Default|GetDartInstance) _returnvalue_2 _returnvalue))))