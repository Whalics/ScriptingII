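; Player ability component for burrowing into allowed surface types at a mana cost, then leaping out.
; Entry checks mana, grounding and surface type via downward trace, or triggers on landing if queued.
; Burrowing lowers the camera through Player-owned timelines, changes capsule collision and friction, and shows breath UI.
; A per-tick sphere trace gates resurfacing and curve-scaled leaps; timer expiry while blocked only prints "Died".
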(event Custom|End%20Timer
  (if (not (Variables|Default|GetbCanResurface))
    (Development|PrintString "Died")))

(event EventBeginPlay
  (|CallParentFunction)
  (CallFunction|SetBurrowData))

(event EventTick
  (params (DeltaSeconds :type Float%20%28single-precision%29))
  (if (Variables|Status|GetbIsBurrowing)
    (CallFunction|CheckCanResurface)))

(fn TrytoBurrow
  (bind _returnvalue (CallFunction|HasMana))
  (if _returnvalue
    (if (not (Variables|Status|GetbIsBurrowing))
      (bind _isburrowable (CallFunction|CheckCanBurrowSurface))
      (if _isburrowable
        (if (Utilities|IsGrounded)
          (Default|DecrementMana (Variables|Default|GetPlayer) (Variables|/Game/DataAssets/PDA_Burrow.PDA_Burrow_C|GetBurrow%20Mana%20Cost (Variables|Data|GetData)))
          (Default|StartBurrow (Variables|Default|GetPlayer) false))))))

(fn CheckCanBurrowSurface
  (bind _player (Variables|Default|GetPlayer))
  (bind _returnvalue (Transformation|GetActorLocation _player))
  (bind _outhit (Collision|LineTraceByChannel _returnvalue (- _returnvalue "0.000000,0.000000,150.000000") "TraceTypeQuery1" false 0 "None"))
  (return (.ReturnValue (Utilities|Map|Find (Variables|Default|GetSurface%20Type) (Collision|GetSurfaceType _outhit)))))

(fn UpdateBurrow
  (params (Alpha :type Float%20%28double-precision%29) (Reverse :type Boolean))
  (Transformation|SetRelativeLocation (Variables|/Game/FirstPerson/Blueprints/BP_FirstPersonCharacter.BP_FirstPersonCharacter_C|GetFirstPersonCamera (Variables|Default|GetPlayer)) (Math|Vector|Lerp(Vector) (Variables|Default|GetStartPosition) (Variables|Default|GetEndPosition) Alpha) false true))

(fn SetBurrowData
  (bind _data (Variables|Data|GetData))
  (Utilities|FlowControl|Sequence
    (:then_0
      (Variables|Data|SetCanLeap (Variables|/Game/DataAssets/PDA_Burrow.PDA_Burrow_C|GetCan%20Leap _data)))
    (:then_1
      (Variables|Data|SetMaxLeapHeight (Variables|/Game/DataAssets/PDA_Burrow.PDA_Burrow_C|GetLeap%20Maximum%20Height _data))
      (Variables|Data|SetMinLeapHeight (Variables|/Game/DataAssets/PDA_Burrow.PDA_Burrow_C|GetLeap%20Minimum%20Height _data)))
    (:then_2
      (Variables|Data|SetLeapManaCost (Variables|/Game/DataAssets/PDA_Burrow.PDA_Burrow_C|GetLeap%20Mana%20Cost _data)))
    (:then_3
      (Variables|Data|SetLeapBreaksWood (Variables|/Game/DataAssets/PDA_Burrow.PDA_Burrow_C|GetLeap%20Breaks%20Wood _data)))
    (:then_4
      (Variables|Data|SetBurrowManaCost (Variables|/Game/DataAssets/PDA_Burrow.PDA_Burrow_C|GetBurrow%20Mana%20Cost _data)))
    (:then_5
      (Variables|Data|SetBurrowMaxDuration (Variables|/Game/DataAssets/PDA_Burrow.PDA_Burrow_C|GetMax%20Duration _data)))
    (:then_6
      (Variables|Data|SetDownSpeed (Variables|/Game/DataAssets/PDA_Burrow.PDA_Burrow_C|GetDown%20Speed _data)))
    (:then_7
      (Variables|Data|SetUpSpeed (Variables|/Game/DataAssets/PDA_Burrow.PDA_Burrow_C|GetUp%20Speed _data)))
    (:then_8
      (Variables|Data|SetbAutomaticUp (Variables|/Game/DataAssets/PDA_Burrow.PDA_Burrow_C|GetAutomatically%20Push%20Up _data)))
    (:then_9
      (Variables|Default|SetFriction (Variables|/Game/DataAssets/PDA_Burrow.PDA_Burrow_C|GetBurrow%20Friction _data)))
    (:then_10
      (Variables|Default|SetBurrow%20Move%20Speed (Variables|/Game/DataAssets/PDA_Burrow.PDA_Burrow_C|GetBurrow%20Movement%20Speed _data)))
    (:then_11
      (Variables|Default|SetBurrowDownFallSpeed (Variables|/Game/DataAssets/PDA_Burrow.PDA_Burrow_C|GetBurrowDownFallSpeed _data)))))

(fn SetupBurrow
  (params (Reverse :type Boolean) (FromFalling :type Boolean))
  (bind _player (Variables|Default|GetPlayer))
  (bind _wbp_hud (Variables|/Game/FirstPerson/Blueprints/BP_FirstPersonCharacter.BP_FirstPersonCharacter_C|GetWBP_HUD _player))
  (bind _wbp_breathbar (Variables|/Game/UI/WBP_HUD.WBP_HUD_C|GetWBP_BreathBar _wbp_hud))
  (if Reverse
    (Default|BreathbarVisibility _wbp_breathbar "Hidden")
    (Variables|/Game/FirstPerson/Blueprints/BP_FirstPersonCharacter.BP_FirstPersonCharacter_C|SetbCanMove (Variables|Default|GetPlayer) true)
    (Default|HideSlider (Variables|/Game/UI/WBP_HUD.WBP_HUD_C|GetWBP_Abilities (Variables|/Game/FirstPerson/Blueprints/BP_FirstPersonCharacter.BP_FirstPersonCharacter_C|GetWBP_HUD (Variables|Default|GetPlayer))))
    (else
      (Default|SetMaxSliderValue _wbp_breathbar (Variables|/Game/DataAssets/PDA_Burrow.PDA_Burrow_C|GetMax%20Duration (Variables|Data|GetData)))
      (Default|BreathbarVisibility (Variables|/Game/UI/WBP_HUD.WBP_HUD_C|GetWBP_BreathBar (Variables|/Game/FirstPerson/Blueprints/BP_FirstPersonCharacter.BP_FirstPersonCharacter_C|GetWBP_HUD (Variables|Default|GetPlayer))) "Visible")
      (Variables|/Game/FirstPerson/Blueprints/BP_FirstPersonCharacter.BP_FirstPersonCharacter_C|SetbCanMove (Variables|Default|GetPlayer) true)
      (Variables|/Script/Engine.CharacterMovementComponent|SetGroundFriction (Variables|Default|GetCharacter%20Movement) (Variables|/Game/DataAssets/PDA_Burrow.PDA_Burrow_C|GetBurrow%20Friction (Variables|Data|GetData)))
      (Variables|Status|SetbIsBurrowing true)
      (Variables|Default|SetStartPosition (Variables|/Script/Engine.SceneComponent|GetRelativeLocation (Variables|/Game/FirstPerson/Blueprints/BP_FirstPersonCharacter.BP_FirstPersonCharacter_C|GetFirstPersonCamera (Variables|Default|GetPlayer))))
      (Variables|Default|SetEndPosition "0.000000,0.000000,-150.000000")
      (Collision|SetCollisionObjectType (Variables|/Script/Engine.Character|GetCapsuleComponent (Variables|Default|GetPlayer)) "ECC_WorldDynamic")
      (if FromFalling
        _
        (else
          (Components|Timeline|SetPlayRate (Variables|/Game/FirstPerson/Blueprints/BP_FirstPersonCharacter.BP_FirstPersonCharacter_C|GetBurrow%20Down%20Timeline (Variables|Default|GetPlayer)) (Variables|/Game/DataAssets/PDA_Burrow.PDA_Burrow_C|GetDown%20Speed (Variables|Data|GetData)))))
      (Components|Timeline|SetPlayRate (Variables|/Game/FirstPerson/Blueprints/BP_FirstPersonCharacter.BP_FirstPersonCharacter_C|GetBurrow%20Up%20Timeline (Variables|Default|GetPlayer)) (Variables|/Game/DataAssets/PDA_Burrow.PDA_Burrow_C|GetUp%20Speed (Variables|Data|GetData)))
      (Variables|Default|SetBurrowTimer (Variables|/Game/DataAssets/PDA_Burrow.PDA_Burrow_C|GetMax%20Duration (Variables|Data|GetData)))
      (Components|Timeline|SetPlayRate (Variables|/Game/FirstPerson/Blueprints/BP_FirstPersonCharacter.BP_FirstPersonCharacter_C|GetBurrowDuration (Variables|Default|GetPlayer)) (/ 1.0 (Variables|/Game/DataAssets/PDA_Burrow.PDA_Burrow_C|GetMax%20Duration (Variables|Data|GetData))))
      (Default|ShowSlider (Variables|/Game/UI/WBP_HUD.WBP_HUD_C|GetWBP_Abilities (Variables|/Game/FirstPerson/Blueprints/BP_FirstPersonCharacter.BP_FirstPersonCharacter_C|GetWBP_HUD (Variables|Default|GetPlayer)))))))

(fn EndBurrow
  (bind _player (Variables|Default|GetPlayer))
  (bind _character_movement (Variables|Default|GetCharacter%20Movement))
  (Collision|SetCollisionObjectType (Variables|/Script/Engine.Character|GetCapsuleComponent (Variables|Default|GetPlayer)) "ECC_Pawn")
  (Variables|Status|SetbIsBurrowing false)
  (Variables|/Game/FirstPerson/Blueprints/BP_FirstPersonCharacter.BP_FirstPersonCharacter_C|SetbCanMove _player true)
  (Variables|/Script/Engine.CharacterMovementComponent|SetGroundFriction _character_movement (Variables|/Game/DataAssets/PDA_General.PDA_General_C|GetDefault%20Friction (Variables|/Game/FirstPerson/Blueprints/BP_FirstPersonCharacter.BP_FirstPersonCharacter_C|GetGeneralData _player)))
  (Variables|/Script/Engine.CharacterMovementComponent|SetMaxWalkSpeed _character_movement (Variables|/Game/DataAssets/PDA_General.PDA_General_C|GetWalk%20Speed (Variables|/Game/FirstPerson/Blueprints/BP_FirstPersonCharacter.BP_FirstPersonCharacter_C|GetGeneralData (Variables|Default|GetPlayer)))))

(fn Landed
  (if (Variables|Default|GetbWaitForLand)
    (Variables|Default|SetbWaitForLand false)
    (Components|Timeline|SetPlayRate (Variables|/Game/FirstPerson/Blueprints/BP_FirstPersonCharacter.BP_FirstPersonCharacter_C|GetBurrow%20Down%20Timeline (Variables|Default|GetPlayer)) (Variables|/Game/DataAssets/PDA_Burrow.PDA_Burrow_C|GetBurrowDownFallSpeed (Variables|Data|GetData)))
    (bind _isburrowable (CallFunction|CheckCanBurrowSurface))
    (if _isburrowable
      (bind _returnvalue (CallFunction|HasMana))
      (if _returnvalue
        (Default|DecrementMana (Variables|Default|GetPlayer) (Variables|/Game/DataAssets/PDA_Burrow.PDA_Burrow_C|GetBurrow%20Mana%20Cost (Variables|Data|GetData)))
        (Default|StartBurrow (Variables|Default|GetPlayer) true)))))

(fn Leap
  (params (InputTime :type Float%20%28double-precision%29))
  (bind _data (Variables|Data|GetData))
  (bind _player (Variables|Default|GetPlayer))
  (if (Variables|Default|GetbCanResurface)
    (Character|LaunchCharacter (Variables|Default|GetPlayer) (Math|Vector|MakeVector 0.0 0.0 (Math|Float|Lerp (Variables|/Game/DataAssets/PDA_Burrow.PDA_Burrow_C|GetLeap%20Minimum%20Height _data) (Variables|/Game/DataAssets/PDA_Burrow.PDA_Burrow_C|GetLeap%20Maximum%20Height _data) (Math|Curves|GetFloatValue (Variables|/Game/DataAssets/PDA_Burrow.PDA_Burrow_C|GetHeight%20Curve (Variables|Data|GetData)) InputTime))) true true)
    (Components|Timeline|SetPlayRate (Variables|/Game/FirstPerson/Blueprints/BP_FirstPersonCharacter.BP_FirstPersonCharacter_C|GetBurrow%20Up%20Timeline (Variables|Default|GetPlayer)) 3.0)
    (CallFunction|EndBurrow)
    (Default|ReverseBurrow _player true)
    (Default|HideSlider (Variables|/Game/UI/WBP_HUD.WBP_HUD_C|GetWBP_Abilities (Variables|/Game/FirstPerson/Blueprints/BP_FirstPersonCharacter.BP_FirstPersonCharacter_C|GetWBP_HUD _player)))))

(fn CheckCanResurface
  (bind _player (Variables|Default|GetPlayer))
  (bind _player_2 (Variables|Default|GetPlayer))
  (bind _returnvalue (Transformation|GetActorLocation _player))
  (bind _returnvalue_2 (Collision|SphereTraceByChannel (- _returnvalue (Math|Vector|MakeVector 0.0 0.0 -2e+01)) (+ _returnvalue (Math|Vector|MakeVector 0.0 0.0 (+ (.z (.OutLocation (Actor|GetActorEyesViewPoint _player_2))) (Variables|/Script/Engine.CapsuleComponent|GetCapsuleHalfHeight (Variables|/Script/Engine.Character|GetCapsuleComponent _player_2))))) (* (Variables|/Script/Engine.CapsuleComponent|GetCapsuleRadius (Variables|/Script/Engine.Character|GetCapsuleComponent (Variables|Default|GetPlayer))) 1.4) "TraceTypeQuery3" false 0 "ForDuration" true "(R=0.000000,G=0.837356,B=1.000000,A=1.000000)" "(R=1.000000,G=0.089091,B=0.000000,A=1.000000)" 2.0))
  (bind _output_get (Variables|Default|SetbCanResurface (not _returnvalue_2)))
  (return _output_get))

(fn SetWaitforLand
  (params (Pressed :type Boolean))
  (Variables|Default|SetbWaitForLand Pressed))

(fn HasMana
  (bind _player (Variables|Default|GetPlayer))
  (bind _currmana (Variables|/Game/FirstPerson/Blueprints/BP_FirstPersonCharacter.BP_FirstPersonCharacter_C|GetCurrMana _player))
  (bind _returnvalue (> _currmana 0))
  (if _returnvalue
    (return _returnvalue)))