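; BP_TargetSpawner spawns BP_Target actors at random points inside a box volume sized by the construction script.
; Activate starts a looping one-second timer on SpawnTarget and immediately spawns an initial cluster.
; SpawnTarget checks CanSpawnTargets, picks a point within half the box extent, turns the target toward the player camera with a yaw offset, and records it in Targets.
; The MaxTargets comparison in CanSpawnTargets is unconnected.
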(event Custom|Spawn%20Target
  (if (Utilities|CanSpawnTargets)
    (bind _output_get (Variables|Default|SetSpawn%20Location (Math|Random|RandomPointinBoundingBox (Transformation|GetWorldLocation (Variables|Default|GetBox)) (/ (Components|Box|GetScaledBoxExtent (Variables|Default|GetBox)) "2.000000,2.000000,2.000000"))))
    (bind _returnvalue (Game|SpawnActorfromClass "/Game/Blueprints/Target/BP_Target.BP_Target_C" (Math|Transform|MakeTransform _output_get (Math|Rotator|MakeRotator (.roll (Math|Rotator|FindLookatRotation _output_get (Transformation|GetWorldLocation (Variables|/Script/Engine.PlayerCameraManager|GetTransformComponent (Game|GetPlayerCameraManager 0))))) (.pitch (Math|Rotator|FindLookatRotation _output_get (Transformation|GetWorldLocation (Variables|/Script/Engine.PlayerCameraManager|GetTransformComponent (Game|GetPlayerCameraManager 0))))) (- (.yaw (Math|Rotator|FindLookatRotation _output_get (Transformation|GetWorldLocation (Variables|/Script/Engine.PlayerCameraManager|GetTransformComponent (Game|GetPlayerCameraManager 0))))) 9e+01)) "1.000000,1.000000,1.000000") "AdjustIfPossibleButAlwaysSpawn" "MultiplyWithRoot" 0 0))
    (Utilities|Array|Add (Variables|Default|GetTargets) _returnvalue)))

(event Custom|Activate
  (Utilities|Time|SetTimerbyEvent (delegate Custom|Spawn%20Target) 1.0 true)
  (CallFunction|SpawnTargetCluster))

(event Custom|Spawn%20Target%20Cluster
  (for _index (range 0 5)
    (CallFunction|SpawnTarget)))

(event EventBeginPlay)

(fn ConstructionScript
  (Components|Box|SetBoxExtent (Variables|Default|GetBox) (Variables|Default|GetIn%20Box%20Extent) true))