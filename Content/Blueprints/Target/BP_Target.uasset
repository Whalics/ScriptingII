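; BP_Target is a damageable target actor that pops in and animates with random variation, and is destroyed when damaged.
; The construction script randomizes start scale and behaviour: horizontal movement, vertical movement or scale adjustment.
; After a random delay, a spawn timeline scales the mesh up at a size-dependent rate, then starts a random-rate timeline driving that behaviour.
; The explosion sound and particle nodes are never run.
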(event EventBeginPlay
  (bind _returnvalue (Math|Random|RandomFloatinRange 5e+01 6e+02))
  (bind _startscale (Variables|Default|GetStartScale))
  (bind _startscale_2 (Variables|Default|GetStartScale))
  (bind _returnvalue_2 (* _startscale_2 1.5))
  (switch Utilities|FlowControl|Switch|SwitchonE_TargetBehaviour (Variables|Default|GetETargetBehaviour)
    (:NewEnumerator1
      (Variables|Default|SetDestinationLocation (Math|Vector|MakeVector _returnvalue 0.0 0.0)))
    (:NewEnumerator2
      (Variables|Default|SetDestinationLocation (Math|Vector|MakeVector 0.0 0.0 _returnvalue)))
    (:NewEnumerator3
      _))
  (Components|Timeline|SetPlayRate (Variables|Default|GetT_Move) (/ 1.0 (Math|Random|RandomFloatinRange 1.5 3.0)))
  (Utilities|FlowControl|Delay (Math|Random|RandomFloatinRange 0.0 1.0))
  (Components|Timeline|SetPlayRate (Variables|Default|GetT_Spawn) (/ 1.0 (Variables|Default|GetStartScale)))
  (bind _alpha (Timeline|T_Spawn PlayFromStart)
    (:Update
      (Transformation|SetWorldScale3D (Variables|Default|GetSM_Target) (Math|Vector|Lerp(Vector) (Math|Vector|MakeVector 0.0 0.0 0.0) (Math|Vector|MakeVector _startscale _startscale _startscale) _alpha)))
    (:Finished
      (bind _alpha_2 (Timeline|T_Move PlayFromStart)
        (:Update
          (switch Utilities|FlowControl|Switch|SwitchonE_TargetBehaviour (Variables|Default|GetETargetBehaviour)
            (:NewEnumerator1
              (Transformation|SetRelativeLocation (Variables|Default|GetSM_Target) (Math|Vector|Lerp(Vector) "0, 0, 0" (Variables|Default|GetDestinationLocation) _alpha_2) true false :!label _label))
            (:NewEnumerator2
              (goto _label))
            (:NewEnumerator3
              (Transformation|SetWorldScale3D (Variables|Default|GetSM_Target) (Math|Vector|Lerp(Vector) (Math|Vector|MakeVector _startscale_2 _startscale_2 1.0) (Math|Vector|MakeVector _returnvalue_2 _returnvalue_2 1.0) _alpha_2)))))))))

(event EventDamaged
  (Actor|DestroyActor))

(fn ConstructionScript
  (Variables|Default|SetStartScale (Math|Random|RandomFloatinRange 0.2 1.0))
  (Variables|Default|SetETargetBehaviour (Utilities|Enum|ByteToEnumE_TargetBehaviour (Math|Conversions|ToByte(Integer) (Math|Random|RandomIntegerinRange 0 2)))))