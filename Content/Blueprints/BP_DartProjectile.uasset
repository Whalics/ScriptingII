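; BP_DartProjectile is a dart projectile actor that damages what it touches and then removes itself.
; A Capsule overlap applies fixed damage to the other actor, plays an attenuated bullet impact sound at the root's location and destroys the dart.
; BeginPlay destroys it after a few seconds as a lifetime limit.
; The Shard hit event is empty, and disconnected leftover nodes for an older damage and destroy path never run.
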(event OnComponentBeginOverlap(Capsule)
  (params (OverlappedComponent :type Primitive%20Component%20Object%20Reference) (OtherActor :type Actor%20Object%20Reference) (OtherComp :type Primitive%20Component%20Object%20Reference) (OtherBodyIndex :type Integer) (bFromSweep :type Boolean) (SweepResult :type Hit%20Result%20Structure%20%28by%20ref%29))
  (Game|Damage|ApplyDamage OtherActor 5e+01 0 0)
  (Audio|PlaySoundatLocation "/Game/Audio/sfx_player_bulletImpact_01.sfx_player_bulletImpact_01" (Transformation|GetWorldLocation (Variables|Default|GetDefaultSceneRoot)) "0, 0, 0" 1.0 1.0 0.0 "/Game/Audio/ATN_Senna.ATN_Senna" 0 0 0)
  (Actor|DestroyActor))

(event OnComponentHit(Shard)
  (params (HitComponent :type Primitive%20Component%20Object%20Reference) (OtherActor :type Actor%20Object%20Reference) (OtherComp :type Primitive%20Component%20Object%20Reference) (NormalImpulse :type Vector :default "0, 0, 0") (Hit :type Hit%20Result%20Structure%20%28by%20ref%29)))

(event EventBeginPlay
  (Utilities|FlowControl|Delay 5.0)
  (Actor|DestroyActor))

(fn ConstructionScript)