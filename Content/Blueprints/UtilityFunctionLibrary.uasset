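; Blueprint function library that turns Enhanced Input actions into button prompt icons and rich text image tags.
; GetButtonPrompt looks up the first player's mapped keys in a key icon table, preferring the Keyboard texture and falling back to any valid platform icon.
; GetRichImageTag uses that texture's asset name as the rich image style row ID to build an img tag.
; Missing table rows print debug messages.
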(fn GetRichImageTag
  (params (InputAction :type Input%20Action%20Object%20Reference))
  (bind ___worldcontext (LocalVariables|Get__WorldContext))
  (bind _returnvalue (CallFunction|GetButtonPrompt InputAction ___worldcontext))
  (bind _returnvalue_2 (Class|KismetSystemLibrary|GetPathName _returnvalue))
  (bind _filenamepart (Utilities|String|Split _returnvalue_2))
  (Utilities|GetDataTableRow "/Game/UI/Fonts/DT_RichImageSytles.DT_RichImageSytles" (Utilities|String|StringToName _filenamepart)
    (:then
      (return (Utilities|Text|FormatText "<img id=\"{id}\" width=\"50\" height=\"50\"></>" _filenamepart)))
    (:RowNotFound
      (Development|PrintString 0 (Utilities|String|Append _filenamepart " is not in image sheet") false))))

(fn GetButtonPrompt
  (params (InputAction :type Input%20Action%20Object%20Reference))
  (for _array_element (Class|EnhancedInputSubsystemInterface|QueryKeysMappedtoAction (PlayerController|LocalPlayerSubsystems|GetEnhancedInputLocalPlayerSubsystem (Game|GetPlayerController (LocalVariables|Get__WorldContext))) InputAction)
    (bind _returnvalue (Utilities|GetDataTableRow "/Game/UI/Sprites/Button_Prompts/DT_KeyIconMap.DT_KeyIconMap" (Utilities|String|StringToName (Utilities|String|ToString(Text) (Class|KismetInputLibrary|KeyGetDisplayName _array_element false))))
      (:then
        (Utilities|IsValid (.Keyboard (Utilities|Struct|BreakF_KeyMappingIcon _returnvalue))
          (:Is%20Valid
            (return (.Keyboard (Utilities|Struct|BreakF_KeyMappingIcon _returnvalue))))
          (:Is%20Not%20Valid
            ;[1 1 1] Return Any texture if correct one isn't found
            (Development|PrintText 0 "Not Valid :(")
            (for _array_element_2 (Utilities|Array|MakeArray (.Keyboard (Utilities|Struct|BreakF_KeyMappingIcon _returnvalue)) (.Xbox (Utilities|Struct|BreakF_KeyMappingIcon _returnvalue)) (.Playstation (Utilities|Struct|BreakF_KeyMappingIcon _returnvalue)))
              (Utilities|IsValid _array_element_2
                (:Is%20Valid
                  (return _array_element_2)))))))
      (:RowNotFound
        (Development|PrintString 0 (Utilities|String|Append (Utilities|String|ToString(Text) (Class|KismetInputLibrary|KeyGetDisplayName _array_element false)) "has not been added to key icon map") false)))))