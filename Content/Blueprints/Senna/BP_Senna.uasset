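; BP_Senna is an actor for Senna that appears and disappears on timed, sound-cued events.
; Appear waits, plays the Q_Senna sound at the actor's location, then shows the mesh with collision, optionally chaining into Disappear.
; Disappear waits, plays the same sound, hides the mesh, disables collision and calls Disappeared.
; On BeginPlay it caches the first-person player character; Freecast simply returns self.
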(event Custom|Disappear
  (params (Delay :type Float%20%28double-precision%29))
  ;[1 1 1] Disappear
  (Utilities|FlowControl|Delay Delay)
  (CallFunction|PlaySound)
  (Utilities|FlowControl|Delay 0.2)
  (Development|SetHiddeninGame (Variables|Default|GetMeshSenna) true false)
  (Collision|SetCollisionEnabled (Variables|Default|GetMeshSenna) "NoCollision")
  (Default|CallDisappeared))

(event Custom|Appear
  (params (Appear%20After :type Float%20%28double-precision%29) (AutoDisappear :type Boolean) (Disappear%20After :type Float%20%28double-precision%29))
  ;[1 1 1] Appear
  (Utilities|FlowControl|Delay Appear%20After)
  (CallFunction|PlaySound)
  (Utilities|FlowControl|Delay 0.1)
  (Development|SetHiddeninGame (Variables|Default|GetMeshSenna) false false)
  (Collision|SetCollisionEnabled (Variables|Default|GetMeshSenna) "QueryAndPhysics")
  (if AutoDisappear
    (CallFunction|Disappear Disappear%20After)))

(event EventBeginPlay
  (bind _asbp_first_person_character (Utilities|Casting|CastToBP_FirstPersonCharacter (Game|Player|GetPlayerPawn 0)))
  (Variables|Default|SetPlayer _asbp_first_person_character))

(event Collision|EventActorBeginOverlap
  (params (OtherActor :type Actor%20Object%20Reference)))

(event EventTick
  (params (DeltaSeconds :type Float%20%28single-precision%29)))

(fn ConstructionScript)

(fn PlaySound
  (Audio|PlaySoundatLocation "/Game/Audio/Q_Senna.Q_Senna" (Transformation|GetActorLocation) "0, 0, 0" 1.0 1.0 0.0 0 0 0 0))

(fn Freecast
  (return self))